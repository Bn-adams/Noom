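; Sun shard resource actor that shows a farm prompt and drops a sun crystal when destroyed.
; Box overlap by a cast-matched actor adds the FarmKey widget; leaving clears all widgets and recreates Player_HUD.
; On destruction it spawns BP_SunCrystal at a random nearby horizontal offset.
; The construction script snaps the actor to a fixed world height, keeping its X and Y.
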(event `self.ReceiveDestroyed`
  (`|SpawnActorFromClass` "/Game/Bps/Resources/BP_SunCrystal.BP_SunCrystal_C" (`KismetMathLibrary.MakeTransform` (`KismetMathLibrary.RandomPointInBoundingBox` (`self.K2_GetActorLocation`) (200.0 200.0 0.0))) "Undefined" "OverrideRootScale" null null))

(event `self.Box.OnComponentBeginOverlap`
  (params (OverlappedComponent :type "PrimitiveComponent Object Reference") (OtherActor :type "Actor Object Reference") (OtherComp :type "PrimitiveComponent Object Reference") (OtherBodyIndex :type Integer) (bFromSweep :type Boolean) (SweepResult :type "HitResult Structure (by ref)"))
  (`|ExecutionSequence`
    (:`then_0`
      (cast `` OtherActor)
      (bind _returnvalue (`|CreateWidget` "/Game/Bps/Interface/FarmKey.FarmKey_C"))
      (`UserWidget.AddToViewport` _returnvalue 0))))

(event `self.Box.OnComponentEndOverlap`
  (params (OverlappedComponent :type "PrimitiveComponent Object Reference") (OtherActor :type "Actor Object Reference") (OtherComp :type "PrimitiveComponent Object Reference") (OtherBodyIndex :type Integer))
  (`|ExecutionSequence`
    (:`then_0`
      (cast `` OtherActor)
      (`WidgetLayoutLibrary.RemoveAllWidgets`)
      (bind _returnvalue (`|CreateWidget` "/Game/Bps/Interface/Player_HUD.Player_HUD_C"))
      (`UserWidget.AddToViewport` _returnvalue 0))))

(fn `UserConstructionScript`
  (bind (_returnvalue_x _returnvalue_y) (`KismetMathLibrary.BreakVector` (`self.K2_GetActorLocation`)))
  (`self.K2_SetActorLocation` (`KismetMathLibrary.MakeVector` _returnvalue_x _returnvalue_y 200.0)))