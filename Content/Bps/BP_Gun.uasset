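; BP_Gun is a gun actor that spawns a BP_Bullet from its ShootSocket shortly after BeginPlay.
; It stores the bullet's movement direction relative to its rotation in NewVar0.
; The velocity override and loop back to the delay are disconnected, so it fires only once.
; A GetPos helper returns a BP_Enemy's location but is not called in this graph.
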(event `self.ReceiveBeginPlay`
  (`KismetSystemLibrary.RetriggerableDelay` 0.4)
  (bind _returnvalue (`|SpawnActorFromClass` "/Game/Bps/Towers/BP_Bullet.BP_Bullet_C" (`KismetMathLibrary.MakeTransform` (`SceneComponent.K2_GetComponentLocation` (`self.Shoot socket`))) "Undefined" "OverrideRootScale" null null))
  (set `self.NewVar_0` (`KismetAnimationLibrary.CalculateDirection` (`self.GetVelocity` _returnvalue) (`self.K2_GetActorRotation` _returnvalue))))

(fn `Get Pos`
  (returns (NewParam :type "Vector Structure"))
  (bind _returnvalue (`GameplayStatics.GetActorOfClass` "/Game/Bps/BP_Enemy.BP_Enemy_C"))
  (return (`self.K2_GetActorLocation` _returnvalue)))

(fn `UserConstructionScript`)