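; BP_Enemy is an enemy that moves along a designer-set path and can be damaged until destroyed.
; The construction script feeds five relative control point positions and a duration into its InterpToMovement component.
; Each Damage event subtracts Pdamage from Health, unless Health already equals exactly zero.
; In that case it destroys the actor, prints a message, sets Dead and clears Overlap.
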(event `Damage`
  (if (== (`self.Health`) 0)
    (`self.K2_DestroyActor`)
    (`KismetSystemLibrary.PrintString` "Enemy Destroyed")
    (set `self.Dead?` true)
    (set `self.Overlap` false)
    (else
      (set `self.Health` (- (`self.Health`) (`self.Pdamage`))))))

(fn `UserConstructionScript`
  (bind _interptomovement (`self.InterpToMovement`))
  (set `InterpToMovementComponent.ControlPoints` (`|MakeArray` (make `InterpControlPoint` (`self.Position Control Point`)) (make `InterpControlPoint` (`self.Position Control Point_0`)) (make `InterpControlPoint` (`self.Position Control Point_1`)) (make `InterpControlPoint` (`self.Position Control Point_2`)) (make `InterpControlPoint` (`self.Position Control Point_3`))) _interptomovement)
  (set `InterpToMovementComponent.Duration` (`self.Duration`) _interptomovement))