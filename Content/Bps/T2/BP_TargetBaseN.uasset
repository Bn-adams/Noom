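; BP_TargetBaseN is a base actor that shoots at and damages a BP_Enemy, likely a turret.
; BeginPlay caches an enemy and calls FaceEnemy, whose interpolated yaw-tracking loop is disconnected and never runs.
; Shoot spawns AmmoType at the Arrow's transform unless the enemy is Dead.
; Damage subtracts PDamage from enemy Health, or destroys this actor, not the enemy, when Health is already zero.
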(event `self.ReceiveBeginPlay`
  (bind _returnvalue (`GameplayStatics.GetActorOfClass` "/Game/Bps/BP_Enemy.BP_Enemy_C"))
  (set `self.EnemyRef` _returnvalue)
  (`self.Face Enemy`))

(event `Face Enemy`)

(fn `Damage`
  (bind _returnvalue (`GameplayStatics.GetActorOfClass` "/Game/Bps/BP_Enemy.BP_Enemy_C"))
  (bind _health (`/Game/Bps/BP_Enemy.Health` _returnvalue))
  (if (== _health 0)
    (`self.K2_DestroyActor`)
    (`KismetSystemLibrary.PrintString` "Enemy Destroyed")
    (else
      (set `/Game/Bps/BP_Enemy.Health` (- _health (`self.PDamage`)) _returnvalue))))

(fn `Shoot`
  (bind _returnvalue (`GameplayStatics.GetActorOfClass` "/Game/Bps/BP_Enemy.BP_Enemy_C"))
  (if (not (`/Game/Bps/BP_Enemy.Dead?` _returnvalue))
    (`|SpawnActorFromClass` (`self.AmmoType`) (`SceneComponent.K2_GetComponentToWorld` (`self.Arrow`)) "Undefined" "OverrideRootScale" null null)))

(fn `UserConstructionScript`)