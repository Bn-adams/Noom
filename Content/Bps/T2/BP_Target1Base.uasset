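; Base Blueprint for what appears to be a turret that shoots BP_Enemy actors entering its Sphere1 range.
; BeginPlay sets the projectile class, caches one enemy reference and calls FaceEnemy once.
; Overlap events toggle the enemy's Overlap flag and start a delay-driven Shoot loop.
; The loop checks the flag on whichever enemy GetActorOfClass returns, not necessarily the one that entered.
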(event `self.ReceiveBeginPlay`
  (`parent.ReceiveBeginPlay`)
  (set `self.AmmoType` "/Game/Bps/Towers/BP_Projectile1.BP_Projectile1_C")
  (bind _returnvalue (`GameplayStatics.GetActorOfClass` "/Game/Bps/BP_Enemy.BP_Enemy_C"))
  (set `self.EnemyRef` _returnvalue)
  (`self.Face Enemy`))

(event `self.Sphere1.OnComponentBeginOverlap`
  (params (OverlappedComponent :type "PrimitiveComponent Object Reference") (OtherActor :type "Actor Object Reference") (OtherComp :type "PrimitiveComponent Object Reference") (OtherBodyIndex :type Integer) (bFromSweep :type Boolean) (SweepResult :type "HitResult Structure (by ref)"))
  (bind _asbp_enemy (cast `/Game/Bps/BP_Enemy` OtherActor))
  (set `/Game/Bps/BP_Enemy.Overlap` true _asbp_enemy)
  (`self.Shoot` :!label _label)
  (`KismetSystemLibrary.Delay` 0.5)
  (bind _returnvalue (`GameplayStatics.GetActorOfClass` "/Game/Bps/BP_Enemy.BP_Enemy_C"))
  (`KismetSystemLibrary.RetriggerableDelay` 0.4)
  (if (`/Game/Bps/BP_Enemy.Overlap` _returnvalue)
    (goto _label)))

(event `self.Sphere1.OnComponentEndOverlap`
  (params (OverlappedComponent :type "PrimitiveComponent Object Reference") (OtherActor :type "Actor Object Reference") (OtherComp :type "PrimitiveComponent Object Reference") (OtherBodyIndex :type Integer))
  (bind _asbp_enemy (cast `/Game/Bps/BP_Enemy` OtherActor))
  (set `/Game/Bps/BP_Enemy.Overlap` false _asbp_enemy))

(fn `UserConstructionScript`
  (`parent.UserConstructionScript`))