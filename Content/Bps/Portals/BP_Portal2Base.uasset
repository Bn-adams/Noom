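; BP_Portal2Base is a portal that teleports the player to a fixed location, apparently back to base.
; Box overlap disables the actor's input and plays a random teleport sound, then after a one-second delay moves the player, restores input and clears BP_Portal2Fight's PassingPortal flag.
; A hard-coded true branch immediately plays both fight and daytime music, so the fight-music stop never runs.
; The construction script pins the portal's height.
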(event `self.Box.OnComponentBeginOverlap`
  (params (OverlappedComponent :type "PrimitiveComponent Object Reference") (OtherActor :type "Actor Object Reference") (OtherComp :type "PrimitiveComponent Object Reference") (OtherBodyIndex :type Integer) (bFromSweep :type Boolean) (SweepResult :type "HitResult Structure (by ref)"))
  (bind _daytime_music_cue (`self.daytime_music_Cue`))
  (bind _level_1_fight_cue (`self.Level_1_fight_Cue`))
  (`|ExecutionSequence`
    (:`then_0`
      (`self.DisableInput` OtherActor null)
      (bind _asbp_player (cast `/Game/Bps/BP_Player` OtherActor))
      (`GameplayStatics.PlaySoundAtLocation` (`KismetArrayLibrary.Array_Random` (`self.TeleportSounds`)) (`self.K2_GetActorLocation` _asbp_player) (struct) 1.0 1.0 0.0 null null null null)
      (`KismetSystemLibrary.Delay` 0.5))
    (:`then_1`
      (`KismetSystemLibrary.Delay` 1.0)
      (bind _asbp_player_2 (cast `/Game/Bps/BP_Player` OtherActor))
      (`self.K2_SetActorLocation` OtherActor (6980.0 -6700.0 200.0) false false)
      (`self.EnableInput` _asbp_player_2 null)
      (bind _returnvalue (`GameplayStatics.GetActorOfClass` "/Game/Bps/Portals/BP_Portal2Fight.BP_Portal2Fight_C"))
      (set `/Game/Bps/Portals/BP_Portal2Fight.passing portal` false _returnvalue))
    (:`then_2`
      ;[1 1 1] Soundtrack nodes - Marv
      (if true
        (`AudioComponent.Play` _level_1_fight_cue 0.0)
        (`AudioComponent.Play` _daytime_music_cue 0.0)
        (else
          (`AudioComponent.Stop` _level_1_fight_cue)
          (`AudioComponent.Play` _daytime_music_cue 0.0))))))

(fn `UserConstructionScript`
  (bind (_returnvalue_x _returnvalue_y) (`KismetMathLibrary.BreakVector` (`self.K2_GetActorLocation`)))
  (`self.K2_SetActorLocation` (`KismetMathLibrary.MakeVector` _returnvalue_x _returnvalue_y 60.0)))