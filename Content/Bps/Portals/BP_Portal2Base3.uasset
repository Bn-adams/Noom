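; BP_Portal2Base3 is a portal actor that sends the player to the NOOMLvl3 level when its box is overlapped.
; On overlap it disables the other actor's input and, for a BP_Player, plays a random teleport sound at the player's location.
; A second sequence branch uses delays to show a loading widget before opening the level by object reference, then calls EnableInput on the player.
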(event `self.Box.OnComponentBeginOverlap`
  (params (OverlappedComponent :type "PrimitiveComponent Object Reference") (OtherActor :type "Actor Object Reference") (OtherComp :type "PrimitiveComponent Object Reference") (OtherBodyIndex :type Integer) (bFromSweep :type Boolean) (SweepResult :type "HitResult Structure (by ref)"))
  (`|ExecutionSequence`
    (:`then_0`
      (`self.DisableInput` OtherActor null)
      (bind _asbp_player (cast `/Game/Bps/BP_Player` OtherActor))
      (`GameplayStatics.PlaySoundAtLocation` (`KismetArrayLibrary.Array_Random` (`self.TeleportSounds`)) (`self.K2_GetActorLocation` _asbp_player) (struct) 1.0 1.0 0.0 null null null null)
      (`KismetSystemLibrary.Delay` 0.5))
    (:`then_1`
      (`KismetSystemLibrary.Delay` 1.0)
      (bind _asbp_player_2 (cast `/Game/Bps/BP_Player` OtherActor))
      (bind _returnvalue (`|CreateWidget` "/Game/Bps/Interface/LoadindWidget.LoadindWidget_C"))
      (`UserWidget.AddToViewport` _returnvalue 0)
      (`KismetSystemLibrary.Delay` 1.0)
      (`GameplayStatics.OpenLevelBySoftObjectPtr` "/Game/Levels/NOOMLvl3.NOOMLvl3")
      (`self.EnableInput` _asbp_player_2 null))))

(fn `UserConstructionScript`)