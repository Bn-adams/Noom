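; BP_TargetBase is a tower base that turns toward an enemy and fires at it.
; From BeginPlay, a self-recalling 0.001-second Delay loop yaws the first BP_TargetBase found toward the BP_Enemy cached at start.
; Shoot spawns AmmoType at the Arrow unless the first enemy found is dead.
; Damage subtracts PDamage from that enemy's Health, or at exactly zero destroys this actor, not the enemy.
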(event `self.ReceiveBeginPlay`
  (bind _returnvalue (`GameplayStatics.GetActorOfClass` "/Game/Bps/BP_Enemy.BP_Enemy_C"))
  (set `self.EnemyRef` _returnvalue)
  (`self.Face Enemy`))

(event `Face Enemy`
  (bind (_returnvalue_roll _returnvalue_pitch _returnvalue_yaw) (`KismetMathLibrary.BreakRotator` (`KismetMathLibrary.RInterpTo` (`self.K2_GetActorRotation`) (`KismetMathLibrary.FindLookAtRotation` (`self.K2_GetActorLocation`) (`self.K2_GetActorLocation` (`self.EnemyRef`))) (`GameplayStatics.GetWorldDeltaSeconds`) 20.0)))
  (bind _returnvalue (`GameplayStatics.GetActorOfClass` "BP_TargetBase_C"))
  (`self.K2_SetActorRotation` _returnvalue (`KismetMathLibrary.MakeRotator` 0.0 0.0 _returnvalue_yaw) false)
  (`KismetSystemLibrary.Delay` 0.001)
  (`self.Face Enemy`))

(fn `Damage`
  (bind _returnvalue (`GameplayStatics.GetActorOfClass` "/Game/Bps/BP_Enemy.BP_Enemy_C"))
  (bind _health (`/Game/Bps/BP_Enemy.Health` _returnvalue))
  (if (== _health 0)
    (`self.K2_DestroyActor`)
    (`KismetSystemLibrary.PrintString` "Enemy Destroyed")
    (else
      (set `/Game/Bps/BP_Enemy.Health` (- _health (`self.PDamage`)) _returnvalue))))

(fn `Shoot`
  (bind _returnvalue (`GameplayStatics.GetActorOfClass` "/Game/Bps/BP_Enemy.BP_Enemy_C"))
  (if (not (`/Game/Bps/BP_Enemy.Dead?` _returnvalue))
    (`|SpawnActorFromClass` (`self.AmmoType`) (`SceneComponent.K2_GetComponentToWorld` (`self.Arrow`)) "Undefined" "OverrideRootScale" null null)))

(fn `UserConstructionScript`)