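; BP_Target1 is a tower that turns to face an enemy and fires BP_Projectile1 from its Arrow component with random bow sounds.
; A self-calling delay loop interpolates yaw toward the BP_Enemy cached at BeginPlay.
; Sphere1 overlaps set the enemy's Overlap flag, driving a delayed repeat of Shoot.
; Shoot, its loop check and Damage use GetActorOfClass rather than the overlapping actor; Damage decrements health or destroys at zero.
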(event `self.ReceiveBeginPlay`
  (bind _returnvalue (`GameplayStatics.GetActorOfClass` "/Game/Bps/BP_Enemy.BP_Enemy_C"))
  (set `self.EnemyRef` _returnvalue)
  (`KismetSystemLibrary.Delay` 0.3)
  (`self.Face Enemy`)
  (set `self.AmmoType` "/Game/Bps/Towers/BP_Projectile1.BP_Projectile1_C")
  (set `self.PDamage` 1))

(event `Face Enemy`
  (bind (_returnvalue_roll _returnvalue_pitch _returnvalue_yaw) (`KismetMathLibrary.BreakRotator` (`KismetMathLibrary.RInterpTo` (`self.K2_GetActorRotation`) (`KismetMathLibrary.FindLookAtRotation` (`self.K2_GetActorLocation`) (`self.K2_GetActorLocation` (`self.EnemyRef`))) (`GameplayStatics.GetWorldDeltaSeconds`) 20.0)))
  (`self.K2_SetActorRotation` (`KismetMathLibrary.MakeRotator` 0.0 0.0 _returnvalue_yaw))
  (`KismetSystemLibrary.Delay` 0.001)
  (`self.Face Enemy`))

(event `self.Sphere1.OnComponentBeginOverlap`
  (params (OverlappedComponent :type "PrimitiveComponent Object Reference") (OtherActor :type "Actor Object Reference") (OtherComp :type "PrimitiveComponent Object Reference") (OtherBodyIndex :type Integer) (bFromSweep :type Boolean) (SweepResult :type "HitResult Structure (by ref)"))
  (bind _asbp_enemy (cast `/Game/Bps/BP_Enemy` OtherActor))
  (set `/Game/Bps/BP_Enemy.Overlap` true _asbp_enemy)
  (`self.Shoot` :!label _label)
  (`KismetSystemLibrary.Delay` 0.5)
  (bind _returnvalue (`GameplayStatics.GetActorOfClass` "/Game/Bps/BP_Enemy.BP_Enemy_C"))
  (`KismetSystemLibrary.RetriggerableDelay` 0.4)
  (if (`/Game/Bps/BP_Enemy.Overlap` _returnvalue)
    (goto _label)))

(event `self.Sphere1.OnComponentEndOverlap`
  (params (OverlappedComponent :type "PrimitiveComponent Object Reference") (OtherActor :type "Actor Object Reference") (OtherComp :type "PrimitiveComponent Object Reference") (OtherBodyIndex :type Integer))
  (bind _asbp_enemy (cast `/Game/Bps/BP_Enemy` OtherActor))
  (set `/Game/Bps/BP_Enemy.Overlap` false _asbp_enemy))

(fn `Damage`
  (bind _returnvalue (`GameplayStatics.GetActorOfClass` "/Game/Bps/BP_Enemy.BP_Enemy_C"))
  (bind _health (`/Game/Bps/BP_Enemy.Health` _returnvalue))
  (if (== _health 0)
    (`self.K2_DestroyActor` _returnvalue)
    (`KismetSystemLibrary.PrintString` "Enemy Destroyed")
    (else
      (set `/Game/Bps/BP_Enemy.Health` (- _health (`self.PDamage`)) _returnvalue))))

(fn `Shoot`
  (`GameplayStatics.PlaySound2D` (`KismetArrayLibrary.Array_Random` (`self.BowSounds`)) 1.0 1.0 0.0 null null)
  (bind _returnvalue (`GameplayStatics.GetActorOfClass` "/Game/Bps/BP_Enemy.BP_Enemy_C"))
  (if (not (`/Game/Bps/BP_Enemy.Dead?` _returnvalue))
    (`|SpawnActorFromClass` (`self.AmmoType`) (`SceneComponent.K2_GetComponentToWorld` (`self.Arrow`)) "Undefined" "OverrideRootScale" null null)))

(fn `UserConstructionScript`)