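; BP_TLVL2P2 is a tower actor, apparently level 2 for P2, that brings its own target and shows a key widget.
; It spawns BP_Target2P2 at its location on BeginPlay, and on destruction removes the first actor of that class found, not a stored reference.
; Its Box adds the P2Lvl1Key widget when a BP_Player enters.
; On exit, it clears all widgets and creates a fresh Player_HUD.
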(event `self.ReceiveBeginPlay`
  (`|SpawnActorFromClass` "/Game/Bps/Towers/P2/BP_Target2P2.BP_Target2P2_C" (`KismetMathLibrary.MakeTransform` (`self.K2_GetActorLocation`)) "Undefined" "OverrideRootScale" null null))

(event `self.ReceiveDestroyed`
  (bind _returnvalue (`GameplayStatics.GetActorOfClass` "/Game/Bps/Towers/P2/BP_Target2P2.BP_Target2P2_C"))
  (`self.K2_DestroyActor` _returnvalue))

(event `self.Box.OnComponentBeginOverlap`
  (params (OverlappedComponent :type "PrimitiveComponent Object Reference") (OtherActor :type "Actor Object Reference") (OtherComp :type "PrimitiveComponent Object Reference") (OtherBodyIndex :type Integer) (bFromSweep :type Boolean) (SweepResult :type "HitResult Structure (by ref)"))
  (`|ExecutionSequence`
    (:`then_0`
      (cast `/Game/Bps/BP_Player` OtherActor)
      (bind _returnvalue (`|CreateWidget` "/Game/Bps/Interface/P2Lvl1Key.P2Lvl1Key_C"))
      (`UserWidget.AddToViewport` _returnvalue 0))))

(event `self.Box.OnComponentEndOverlap`
  (params (OverlappedComponent :type "PrimitiveComponent Object Reference") (OtherActor :type "Actor Object Reference") (OtherComp :type "PrimitiveComponent Object Reference") (OtherBodyIndex :type Integer))
  (`|ExecutionSequence`
    (:`then_0`
      (cast `/Game/Bps/BP_Player` OtherActor)
      (`WidgetLayoutLibrary.RemoveAllWidgets`)
      (bind _returnvalue (`|CreateWidget` "/Game/Bps/Interface/Player_HUD.Player_HUD_C"))
      (`UserWidget.AddToViewport` _returnvalue 0))))

(fn `UserConstructionScript`)