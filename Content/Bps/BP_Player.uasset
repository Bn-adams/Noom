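; Player character that walks on a flat plane, gathers wood, stone and sun shards, and upgrades towers.
; Key presses set an animation state, which Tick turns into Paper2D flipbooks.
; Farming briefly disables input and destroys overlapped trees, rocks and shards, while capsule overlaps count pickups and flag build zones.
; Three build-check events test resources, swap overlapped towers for the next level, and deduct only wood and stone.
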(event `InputAction|Cheats`
  (params (Key :type "Key Structure"))
  ;[1 1 1] Cheats
  (:`Pressed`
    (set `self.WoodCount` (+ (`self.WoodCount`) 1))
    (set `self.StoneCount` (+ (`self.StoneCount`) 1))
    (set `self.SunShardCount` (+ (`self.SunShardCount`) 1))))

(event `lock Z`
  (bind (_returnvalue_x _returnvalue_y) (`KismetMathLibrary.BreakVector` (`self.K2_GetActorLocation`)))
  ;[1 1 1] NO overlaps
  (`self.K2_SetActorLocation` (`KismetMathLibrary.MakeVector` _returnvalue_x _returnvalue_y 150.0)))

(event `self.ReceiveBeginPlay`
  (bind _returnvalue (`GameplayStatics.GetPlayerController` 0))
  ;[1 1 1] Show mouse
  (set `PlayerController.bShowMouseCursor` true _returnvalue)
  (set `PlayerController.bEnableMouseOverEvents` true _returnvalue))

(event `self.ReceiveTick`
  (params (DeltaSeconds :type "Float (single-precision)"))
  (`self.AnimationHandler`))

(event `InputAxis|MoveRight`
  (params (AxisValue :type "Float (single-precision)"))
  ;[1 1 1] Player Movement
  (`self.AddMovementInput` (1.0 0.0 0.0) AxisValue))

(event `InputAxis|MoveUP`
  (params (AxisValue :type "Float (single-precision)"))
  ;[1 1 1] Player Movement
  (`self.AddMovementInput` (0.0 1.0 0.0) AxisValue))

(event `Key|D`
  (params (Key :type "Key Structure"))
  ;[1 1 1] Animation for Player
  (:`Pressed`
    (set `self.AniState` "NewEnumerator2"))
  (:`Released`
    (set `self.AniState` "NewEnumerator4")))

(event `AnimationHandler`
  ;[1 1 1] Animation for Player
  (switch `/Game/Assets/Players/Animation` (`self.AniState`)
    (:`NewEnumerator0`
      (`PaperFlipbookComponent.SetFlipbook` (`self.Sprite`) "/Game/Assets/Players/FB_Player_Up.FB_Player_Up"))
    (:`NewEnumerator1`
      (`PaperFlipbookComponent.SetFlipbook` (`self.Sprite`) "/Game/Assets/Players/FB_Player_Down.FB_Player_Down"))
    (:`NewEnumerator2`
      (`PaperFlipbookComponent.SetFlipbook` (`self.Sprite`) "/Game/Assets/Players/FB_Player_Right.FB_Player_Right"))
    (:`NewEnumerator3`
      (`PaperFlipbookComponent.SetFlipbook` (`self.Sprite`) "/Game/Assets/Players/FB_Player_left.FB_Player_left"))
    (:`NewEnumerator4`
      (`PaperFlipbookComponent.SetFlipbook` (`self.Sprite`) "/Game/Assets/Players/FB_Idle_down.FB_Idle_down"))
    (:`NewEnumerator5`
      (`PaperFlipbookComponent.SetFlipbook` (`self.Sprite`) "/Game/Assets/Players/Axe.Axe"))))

(event `Key|A`
  (params (Key :type "Key Structure"))
  ;[1 1 1] Animation for Player
  (:`Pressed`
    (set `self.AniState` "NewEnumerator3"))
  (:`Released`
    (set `self.AniState` "NewEnumerator4")))

(event `Key|S`
  (params (Key :type "Key Structure"))
  ;[1 1 1] Animation for Player
  (:`Pressed`
    (set `self.AniState` "NewEnumerator1"))
  (:`Released`
    (set `self.AniState` "NewEnumerator4")))

(event `Key|W`
  (params (Key :type "Key Structure"))
  ;[1 1 1] Animation for Player
  (:`Pressed`
    (set `self.AniState` "NewEnumerator0"))
  (:`Released`
    (set `self.AniState` "NewEnumerator4")))

(event `self.CapsuleComponent.OnComponentEndOverlap`
  (params (OverlappedComponent :type "PrimitiveComponent Object Reference") (OtherActor :type "Actor Object Reference") (OtherComp :type "PrimitiveComponent Object Reference") (OtherBodyIndex :type Integer))
  ;[1 1 1] Set not in build zone
  (cast `/Game/Bps/Towers/BP_TLVL0` OtherActor
    (:`then`
      (set `self.PlayerInBuild` 0))
    (:`CastFailed`
      (cast `/Game/Bps/Towers/TLVL1` OtherActor
        (:`then`
          (set `self.PlayerInBuild` 0))
        (:`CastFailed`
          (cast `/Game/Bps/Towers/TLVL2` OtherActor)
          (set `self.PlayerInBuild` 0))))))

(event `self.CapsuleComponent.OnComponentBeginOverlap`
  (params (OverlappedComponent :type "PrimitiveComponent Object Reference") (OtherActor :type "Actor Object Reference") (OtherComp :type "PrimitiveComponent Object Reference") (OtherBodyIndex :type Integer) (bFromSweep :type Boolean) (SweepResult :type "HitResult Structure (by ref)"))
  ;[1 1 1] Resource Counters
  (`|ExecutionSequence`
    (:`then_0`
      (cast `/Game/Bps/Resources/BP_Wood` OtherActor
        (:`then`
          (set `self.WoodCount` (+ (`self.WoodCount`) 1))
          (`GameplayStatics.PlaySound2D` "/Game/Assets/Sounds/Foley/Pop.Pop" 1.0 1.0 0.0 null null))
        (:`CastFailed`
          (cast `/Game/Bps/Resources/BP_Stone` OtherActor
            (:`then`
              (set `self.StoneCount` (+ (`self.StoneCount`) 1))
              (`GameplayStatics.PlaySound2D` "/Game/Assets/Sounds/Foley/Pop.Pop" 1.0 1.0 0.0 null null))
            (:`CastFailed`
              (cast `/Game/Bps/Resources/BP_SunCrystal` OtherActor)
              (set `self.SunShardCount` (+ (`self.SunShardCount`) 1))
              (`GameplayStatics.PlaySound2D` "/Game/Assets/Sounds/Foley/Pop.Pop" 1.0 1.0 0.0 null null))))))
    (:`then_1`
      ;[1 1 1] Set in build zone
      (cast `/Game/Bps/Towers/BP_TLVL0` OtherActor
        (:`then`
          (set `self.PlayerInBuild` 1))
        (:`CastFailed`
          (cast `/Game/Bps/Towers/TLVL1` OtherActor
            (:`then`
              (set `self.PlayerInBuild` 1))
            (:`CastFailed`
              (cast `/Game/Bps/Towers/TLVL2` OtherActor)
              (set `self.PlayerInBuild` 1))))))))

(event `InputAction|farming`
  (params (Key :type "Key Structure"))
  (bind _returnvalue (`GameplayStatics.GetPlayerController` 0))
  ;[1 1 1] Farming system
  (:`Pressed`
    (`self.DisableInput` _returnvalue)
    (`KismetSystemLibrary.Delay` 0.1)
    (set `self.AniState` "NewEnumerator5")
    (`GameplayStatics.PlaySoundAtLocation` "/Game/Assets/Sounds/Foley/Chop_1.Chop_1" (`self.K2_GetActorLocation` _returnvalue) (struct) 1.0 1.0 0.0 null null null null)
    (`KismetSystemLibrary.Delay` 0.5)
    (`self.EnableInput` _returnvalue)
    (`|ExecutionSequence`
      (:`then_0`
        ;;[1 1 1] Wood
        (for _array_element (`self.GetOverlappingActors` "/Game/Bps/Resources/BP_Tree.BP_Tree_C")
          (`KismetSystemLibrary.Delay` 0.5)
          (`self.K2_DestroyActor` _array_element)))
      (:`then_1`
        ;;[1 1 1] Stone
        (for _array_element_2 (`self.GetOverlappingActors` "/Game/Bps/Resources/BP_Rock.BP_Rock_C")
          (`KismetSystemLibrary.Delay` 0.5)
          (`self.K2_DestroyActor` _array_element_2)))
      (:`then_2`
        ;;[1 1 1] SunShard
        (for _array_element_3 (`self.GetOverlappingActors` "/Game/Bps/Resources/BP_SunShard.BP_SunShard_C")
          (`KismetSystemLibrary.Delay` 0.5)
          (`self.K2_DestroyActor` _array_element_3))))))

(event `LvL0BuildCheck`
  ;[1 1 1] Tower Building
  (if (> (`self.PlayerInBuild`) 0)
    (if (>= (`self.StoneCount`) 2)
      (if (>= (`self.WoodCount`) 3)
        (bind _returnvalue (`GameplayStatics.GetActorOfClass` "BP_Player_C"))
        (for _array_element (`self.GetOverlappingActors` _returnvalue "/Game/Bps/Towers/BP_TLVL0.BP_TLVL0_C")
          (bind _asbp_tlvl0 (cast `/Game/Bps/Towers/BP_TLVL0` _array_element))
          (`|SpawnActorFromClass` "/Game/Bps/Towers/TLVL1.TLVL1_C" (`KismetMathLibrary.Conv_VectorToTransform` (`self.K2_GetActorLocation` _asbp_tlvl0)) "Undefined" "OverrideRootScale" null null)
          (`self.K2_DestroyActor` _array_element)
          (set `self.WoodCount` (- (`self.WoodCount`) 3))
          (set `self.StoneCount` (- (`self.StoneCount`) 2)))
        (else
          (`KismetSystemLibrary.PrintString` "You need more stuff" :!label _label)))
      (else
        (goto _label)))))

(event `Lvl1BuildCheck`
  ;[1 1 1] Tower Building
  (if (>= (`self.PlayerInBuild`) 0)
    (if (>= (`self.SunShardCount`) 3)
      (if (>= (`self.StoneCount`) 2)
        (if (>= (`self.WoodCount`) 3)
          (bind _returnvalue (`GameplayStatics.GetActorOfClass` "BP_Player_C"))
          (for _array_element (`self.GetOverlappingActors` _returnvalue "/Game/Bps/Towers/TLVL1.TLVL1_C")
            (bind _astlvl1 (cast `/Game/Bps/Towers/TLVL1` _array_element))
            (`|SpawnActorFromClass` "/Game/Bps/Towers/TLVL2.TLVL2_C" (`KismetMathLibrary.Conv_VectorToTransform` (`self.K2_GetActorLocation` _astlvl1)) "Undefined" "OverrideRootScale" null null)
            (`self.K2_DestroyActor` _array_element)
            (set `self.WoodCount` (- (`self.WoodCount`) 3))
            (set `self.StoneCount` (- (`self.StoneCount`) 2))))))))

(event `BuildCheckLvl2`
  ;[1 1 1] Tower Building
  (if (>= (`self.PlayerInBuild`) 0)
    (if (>= (`self.SunShardCount`) 3)
      (if (>= (`self.StoneCount`) 2)
        (if (>= (`self.WoodCount`) 3)
          (bind _returnvalue (`GameplayStatics.GetActorOfClass` "BP_Player_C"))
          (for _array_element (`self.GetOverlappingActors` _returnvalue "/Game/Bps/Towers/TLVL2.TLVL2_C")
            (bind _astlvl2 (cast `/Game/Bps/Towers/TLVL2` _array_element))
            (`|SpawnActorFromClass` "/Game/Bps/Towers/TLVL3.TLVL3_C" (`KismetMathLibrary.Conv_VectorToTransform` (`self.K2_GetActorLocation` _astlvl2)) "Undefined" "OverrideRootScale" null null)
            (`self.K2_DestroyActor` _array_element)
            (set `self.WoodCount` (- (`self.WoodCount`) 3))
            (set `self.StoneCount` (- (`self.StoneCount`) 2))))))))

(fn `UserConstructionScript`
  (bind (_returnvalue_x _returnvalue_y) (`KismetMathLibrary.BreakVector` (`self.K2_GetActorLocation`)))
  (`self.K2_SetActorLocation` (`KismetMathLibrary.MakeVector` _returnvalue_x _returnvalue_y 200.0)))