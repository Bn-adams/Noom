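; BP_Tower is a tower actor that damages BP_Enemy actors within its overlap range.
; Begin overlap sets the enemy's Overlap flag, then loops Damage calls through a retriggerable delay until that flag clears.
; End overlap clears the flag only if the enemy still has health.
; The loop shares one delay and one cast result, so a newly entering enemy takes over the damage ticks from the previous one.
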(event `self.ReceiveActorBeginOverlap`
  (params (OtherActor :type "Actor Object Reference"))
  (bind _asbp_enemy (cast `/Game/Bps/BP_Enemy` OtherActor))
  (set `/Game/Bps/BP_Enemy.Overlap` true _asbp_enemy)
  (`KismetSystemLibrary.PrintString` "Enemy spotted")
  (bind _asbp_enemy_2 (cast `/Game/Bps/BP_Enemy` OtherActor))
  (`/Game/Bps/BP_Enemy.Damage` _asbp_enemy_2 :!label _label)
  (if (`/Game/Bps/BP_Enemy.Overlap` _asbp_enemy_2)
    (`KismetSystemLibrary.RetriggerableDelay` 0.5)
    (goto _label)))

(event `self.ReceiveActorEndOverlap`
  (params (OtherActor :type "Actor Object Reference"))
  (bind _asbp_enemy (cast `/Game/Bps/BP_Enemy` OtherActor))
  (if (> (`/Game/Bps/BP_Enemy.Health` _asbp_enemy) 0)
    (bind _asbp_enemy_2 (cast `/Game/Bps/BP_Enemy` OtherActor))
    (set `/Game/Bps/BP_Enemy.Overlap` false _asbp_enemy_2)
    (`KismetSystemLibrary.PrintString` "Enemy out of range")))

(fn `UserConstructionScript`)