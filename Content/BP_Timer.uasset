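; BP_Timer is a countdown timer actor that prints its remaining time to the screen once per second.
; On BeginPlay it prints a start message, then calls the StartTimer event, which prints Time and decrements it.
; A branch feeds a one-second Retriggerable Delay back into StartTimer, looping while Time stays at or above zero.
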(event `StartTimer`
  ;[1 1 1] Prints the time & minuses 1 from it
  (`KismetSystemLibrary.PrintString` (`KismetStringLibrary.Conv_IntToString` (`self.Time`)))
  (set `self.Time` (- (`self.Time`) 1)))

(event `self.ReceiveBeginPlay`
  ;[1 1 1] When called, it calles the StartTimer function every second until it reaches zero
  (`KismetSystemLibrary.PrintString` "timer start")
  (`self.StartTimer` :!label _label)
  (if (>= (`self.Time`) 0)
    (`KismetSystemLibrary.RetriggerableDelay` 1.0)
    (goto _label)))

(fn `UserConstructionScript`)